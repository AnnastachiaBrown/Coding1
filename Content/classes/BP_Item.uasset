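; BP_Item is an item actor that sets its damage by type (weapon, tool or consumable) and attacks an enemy.
; On BeginPlay, Constructor rolls weapon damage and picks a random name for unnamed weapons, then prints both.
; After a delay, Atatck targets the first BP_Enemy found, but multiplies damage by zero, leaving Health unchanged.
; A timeline also moves the cube vertically through a Lerp on its relative Z.
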(event EventBeginPlay
  (Utilities|FlowControl|Sequence
    (:then_0
      (CallFunction|Constructor)
      (Development|PrintString (Utilities|String|Append "name: " (Variables|Default|Getname) "  Damage: " (Utilities|String|ToString(Integer) (Variables|Default|Getdamage))) true true "(R=0.000000,G=0.660000,B=1.000000,A=1.000000)" 5.0)
      (Utilities|FlowControl|Delay 5.0)
      (bind _returnvalue (Actor|GetActorOfClass "/Game/Blueprint/BP_Enemy.BP_Enemy_C"))
      (CallFunction|Atatck _returnvalue))
    (:then_1
      (bind _newtrack_0 (Timeline|Timeline Play)
        (:Update
          (Transformation|SetRelativeLocation (Variables|Default|GetCube) (Math|Vector|MakeVector 0.0 0.0 (Math|Float|Lerp 0.0 1e+02 _newtrack_0)) false false))))))

(event Collision|EventActorBeginOverlap
  (params (OtherActor :type Actor%20Object%20Reference)))

(event EventTick
  (params (DeltaSeconds :type Float%20%28single-precision%29)))

(fn ConstructionScript)

(fn Constructor
  (bind _weaponnames (Variables|Default|GetweaponNames))
  (switch Utilities|FlowControl|Switch|SwitchonItemType (Variables|Default|GetType)
    (:NewEnumerator0
      (Variables|Default|Setdamage (Math|Random|RandomIntegerinRange 3 6))
      (if (Utilities|Enum|Equal(Enum) (Variables|Default|Getname) "") ; if true randomize name
        (Utilities|Array|Shuffle _weaponnames)
        (Variables|Default|Setname (Utilities|Array|Get(acopy) _weaponnames))))
    (:NewEnumerator1
      (Variables|Default|Setdamage 1))
    (:NewEnumerator2
      (Variables|Default|Setdamage 0))))

(fn Atatck
  (params (GivenEnemy :type BP%20Enemy%20Object%20Reference))
  (Variables|/Game/Blueprint/BP_Enemy.BP_Enemy_C|SetHealth GivenEnemy (- (Variables|/Game/Blueprint/BP_Enemy.BP_Enemy_C|GetHealth GivenEnemy) (* (Math|Conversions|ToFloat(Integer) (Variables|Default|Getdamage)) 0.0))))