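; BP_EnemySpawner populates the level with BP_Enemy actors and starts a new wave once none remain.
; On BeginPlay it gathers all BP_EnemySpawnLocation actors, prints their count and spawns the first wave.
; Each location has an 80% chance to spawn an enemy at its transform.
; A self-calling event with a Delay polls every two seconds using GetAllActorsOfClass, a cost the author's comments acknowledge, and respawns when the count is zero.
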(event Custom|Spawn%20Enimes
  (for _array_element (stale EventBeginPlay _outactors)
    (if (< (Math|Random|RandomFloat) 0.8)
      (Game|SpawnActorfromClass "/Game/Blueprint/BP_Enemy.BP_Enemy_C" (Transformation|GetActorTransform _array_element) "Undefined" "MultiplyWithRoot" 0 0) ; Spawn actor from class
    )))

(event Custom|CheckEnemyCount
  (bind _outactors (Actor|GetAllActorsOfClass "/Game/Blueprint/BP_Enemy.BP_Enemy_C")) ; this is rescource expensive not optimal but works
  (if (> (Utilities|Array|Length _outactors) 0) ; if length is 0 than the action if false
    _
    (else
      (CallFunction|SpawnEnimes)))
  (Utilities|FlowControl|Delay 2.0)
  (CallFunction|CheckEnemyCount))

(event EventBeginPlay
  (bind _outactors (Actor|GetAllActorsOfClass "/Game/Blueprint/BP_EnemySpawnLocation.BP_EnemySpawnLocation_C"))
  (Development|PrintString (Utilities|String|Append " There are " (Utilities|String|ToString(Integer) (Utilities|Array|Length _outactors)) " spawn locations!") true true "(R=1.000000,G=0.919861,B=0.397387,A=1.000000)" 1e+01)
  (CallFunction|SpawnEnimes)
  (CallFunction|CheckEnemyCount))

(fn ConstructionScript)