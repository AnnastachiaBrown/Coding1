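; BP_Key is a key pickup that the player collects by running into it.
; A hit on its Sphere component casts the other actor to BP_ThirdPersonCharacter and increments that character's TotalKeys.
; It then plays a powerup sound, destroys itself and prints the total as a debug check.
; TotalKeys is capped at ten only after that print, so the message can show a value over the limit.
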(event OnComponentHit(Sphere)
  (params (HitComponent :type Primitive%20Component%20Object%20Reference) (OtherActor :type Actor%20Object%20Reference) (OtherComp :type Primitive%20Component%20Object%20Reference) (NormalImpulse :type Vector :default "0, 0, 0") (Hit :type Hit%20Result%20Structure%20%28by%20ref%29))
  (bind _asbp_third_person_character (Utilities|Casting|CastToBP_ThirdPersonCharacter OtherActor)) ; Was it the player that ran into us
  (Math|Integer|IncrementInt (Variables|/Game/ThirdPerson/Blueprints/BP_ThirdPersonCharacter.BP_ThirdPersonCharacter_C|GettotalKeys _asbp_third_person_character)
    (:%20%20
      (Audio|SpawnSoundatLocation "/Game/Audio/Powerup2_Cue.Powerup2_Cue" (Transformation|GetWorldLocation (Variables|Default|GetDefaultSceneRoot)) "0, 0, 0" 1.0 1.0 0.0 0 0)
      (Actor|DestroyActor) ; "pick up" the key
      (Development|PrintString (Utilities|String|Append "Total Keys = " (Utilities|String|ToString(Integer) (Variables|/Game/ThirdPerson/Blueprints/BP_ThirdPersonCharacter.BP_ThirdPersonCharacter_C|GettotalKeys _asbp_third_person_character)))) ; a way to test
      (if (> (Variables|/Game/ThirdPerson/Blueprints/BP_ThirdPersonCharacter.BP_ThirdPersonCharacter_C|GettotalKeys _asbp_third_person_character) 10) ; limit total keys
        (Variables|/Game/ThirdPerson/Blueprints/BP_ThirdPersonCharacter.BP_ThirdPersonCharacter_C|SettotalKeys _asbp_third_person_character 10) ; Set the Total Keys
      ))))

(event EventBeginPlay)

(event Collision|EventActorBeginOverlap
  (params (OtherActor :type Actor%20Object%20Reference)))

(event EventTick
  (params (DeltaSeconds :type Float%20%28single-precision%29)))

(fn ConstructionScript)