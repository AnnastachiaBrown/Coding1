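; BP_Enemy is an enemy actor that dies with an explosion sound when the player character runs into it.
; A capsule overlap with BP_ThirdPersonCharacter sets Health below zero directly, with no incremental damage.
; From BeginPlay, the CheckHealth event re-calls itself after a short delay as a polling loop.
; Once Health is negative, the loop plays a 2D sound and destroys the actor.
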(event OnComponentBeginOverlap(Capsule)
  (params (OverlappedComponent :type Primitive%20Component%20Object%20Reference) (OtherActor :type Actor%20Object%20Reference) (OtherComp :type Primitive%20Component%20Object%20Reference) (OtherBodyIndex :type Integer) (bFromSweep :type Boolean) (SweepResult :type Hit%20Result%20Structure%20%28by%20ref%29))
  (Utilities|Casting|CastToBP_ThirdPersonCharacter OtherActor) ; if player runs into enemy
  (Variables|Default|SetHealth -1.0) ; set health
)

(event Custom|Check%20health
  (Utilities|FlowControl|Delay 0.2) ; delays action by .2
  (if (>= (Variables|Default|GetHealth) 0.0) ; if statement
    (CallFunction|CheckHealth) ; loops every .2 seconds
    (else
      (Audio|SpawnSound2D "/Game/Audio/Explosion5.Explosion5" 1.0 1.0 0.0 0)
      (Actor|DestroyActor) ; Object Dies
    )))

(event EventBeginPlay
  (CallFunction|CheckHealth) ; starts the loop of checking heakth
)

(event Collision|EventActorBeginOverlap
  (params (OtherActor :type Actor%20Object%20Reference)))

(event EventTick
  (params (DeltaSeconds :type Float%20%28single-precision%29)))

(fn ConstructionScript)